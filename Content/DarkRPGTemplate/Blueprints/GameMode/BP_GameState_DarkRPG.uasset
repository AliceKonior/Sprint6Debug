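; Game state for the Dark RPG template that resets every NPC in the level when the player dies.
; On BeginPlay it binds ResetNPCs to the death event of the BP_Player character, which passes each BP_NPC_base actor to ReplaceNPC.
; ReplaceNPC destroys the NPC and respawns its class at its initial transform, carrying over patrol and drop settings but always assigning the zombie behavior tree.
; The remaining functions are stubs returning defaults.
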(event Custom|ResetNPCs
  (bind _outactors (Actor|GetAllActorsOfClass "/Game/DarkRPGTemplate/Blueprints/Characters/BP_NPC_base.BP_NPC_base_C")) ; Get all NPCs in the level
  (for _array_element _outactors ; Loop through them
    (CallFunction|ReplaceNPC _array_element) ; And call on them to be replaced
  ))

(event EventBeginPlay
  (bind _asbp_player (Utilities|Casting|CastToBP_Player (Game|GetPlayerCharacter 0)))
  (EventDispatchers|BindEventtoPlayerDeath _asbp_player (delegate Custom|ResetNPCs)) ; Bind ResetNPCs event to when the player\ndies
)

(fn ConstructionScript)

(fn ReplaceNPC
  (params (OldNPC :type BP%20NPC%20Base%20Object%20Reference))
  ;[1 1 1] Save NPC's public variables
  (bind _output_get (LocalVariables|SetLocalOldNPC OldNPC))
  (LocalVariables|SetLocalShouldPatrol (Variables|/Game/DarkRPGTemplate/Blueprints/Characters/BP_NPC_base.BP_NPC_base_C|GetShouldPatrol _output_get))
  (LocalVariables|SetLocalItemsToDrop (Variables|/Game/DarkRPGTemplate/Blueprints/Characters/BP_NPC_base.BP_NPC_base_C|GetItemsToDrop (LocalVariables|GetLocalOldNPC)))
  (LocalVariables|SetLocalChanceToDrop (Variables|/Game/DarkRPGTemplate/Blueprints/Characters/BP_NPC_base.BP_NPC_base_C|GetChanceToDrop (LocalVariables|GetLocalOldNPC)))
  (LocalVariables|SetLocalClass (Utilities|GetClass (LocalVariables|GetLocalOldNPC)))
  (LocalVariables|SetLocalInitalTransform (Variables|/Game/DarkRPGTemplate/Blueprints/Characters/BP_NPC_base.BP_NPC_base_C|GetInitialTransform (LocalVariables|GetLocalOldNPC)))
  (Class|Pawn|DetachfromControllerPendingDestroy (LocalVariables|GetLocalOldNPC)) ; Detatch the AI controller before destroying\nthe NPC
  (Actor|DestroyActor (LocalVariables|GetLocalOldNPC))
  (bind _returnvalue (AI|SpawnAIFromClass (LocalVariables|GetLocalClass) "/Game/DarkRPGTemplate/Blueprints/AI/Zombie/BehaviourTree_Zombie.BehaviourTree_Zombie" (.Location (Math|Transform|BreakTransform (LocalVariables|GetLocalInitalTransform))) (.Rotation (Math|Transform|BreakTransform (LocalVariables|GetLocalInitalTransform))) true)) ; Spawn a new NPC of the same class, at the old NPC's\ninitial transform
  (bind _asbp_npc_base (Utilities|Casting|CastToBP_NPC_base _returnvalue))
  (LocalVariables|SetLocalNewNPC _asbp_npc_base)
  ;[1 1 1] Set new NPC's public variables
  (Variables|/Game/DarkRPGTemplate/Blueprints/Characters/BP_NPC_base.BP_NPC_base_C|SetShouldPatrol (LocalVariables|GetLocalNewNPC) (LocalVariables|GetLocalShouldPatrol))
  (Variables|/Game/DarkRPGTemplate/Blueprints/Characters/BP_NPC_base.BP_NPC_base_C|SetItemsToDrop (LocalVariables|GetLocalNewNPC) (LocalVariables|GetLocalItemsToDrop))
  (Variables|/Game/DarkRPGTemplate/Blueprints/Characters/BP_NPC_base.BP_NPC_base_C|SetChanceToDrop (LocalVariables|GetLocalNewNPC) (LocalVariables|GetLocalChanceToDrop)))

(fn ActorCanBleed
  (return false))

(fn AddtoUserInventory
  (params (InventoryItem :type BP%20Inventory%20Item%20Class%20Reference))
  (return false))

(fn Begin/EndPray
  (params (Begin :type Boolean))
  (return 0.0))

(fn GetFaction
  (return "NewEnumerator0"))

(fn GetIsDead
  (return false))

(fn GetTorsoMontage
  (return false))

(fn GetWeapon
  (return 0))

(fn GetXPWorth
  (return 0))