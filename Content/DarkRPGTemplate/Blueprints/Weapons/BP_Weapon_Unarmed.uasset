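; BP_Weapon_Unarmed is the unarmed weapon Blueprint, providing the hit detection for attacks made without a weapon.
; Its CollisionTrace function sweeps a single sphere of TraceRadius between the DamageTrace01 and DamageTrace02 points and returns the hit result.
; The trace ignores actors in HitActors and draws no debug shapes.
; The event graph holds no active logic, and the construction script only calls its parent.
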(event EventBeginPlay)

(event Collision|EventActorBeginOverlap
  (params (OtherActor :type Actor%20Object%20Reference)))

(event EventTick
  (params (DeltaSeconds :type Float%20%28single-precision%29))
  (|CallParentFunction 0.0))

(fn ConstructionScript
  (|CallParentFunction))

(fn CollisionTrace
  (bind _outhit (Collision|SphereTraceByChannel (Transformation|GetWorldLocation (Variables|Default|GetDamageTrace01)) (Transformation|GetWorldLocation (Variables|Default|GetDamageTrace02)) (Variables|Default|GetTraceRadius) "TraceTypeQuery3" false (Variables|Default|GetHitActors) "None"))
  (return _outhit))