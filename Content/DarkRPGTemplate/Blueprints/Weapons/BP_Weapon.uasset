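; Melee weapon actor that deals point damage during swings and awards the owner XP for kills.
; Begin/EndSwing opens a Tick gate for line or sphere traces between two points, behind a second gate that disables the weapon.
; An ignore list prevents repeat hits on pawns within one swing.
; Pawn hits play gore effects; active shields and other solid objects stagger the owner and end the swing, using interface messages.
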(event Custom|OpenSwingGate
  (Utilities|FlowControl|Gate true) ; enters at Open
)

(event Custom|CloseSwingGate
  (Utilities|Array|Clear (Variables|Default|GetHitActors)) ; Reset the hit actors when\nwe stop swinging
  (Utilities|Array|Add (Variables|Default|GetHitActors) (Actor|GetParentActor)) ; Add back the parent
  (Utilities|FlowControl|Gate true) ; enters at Close
)

(event Custom|EnableWeapon
  (Utilities|FlowControl|Gate false) ; enters at Open
)

(event Custom|DisableWeapon
  (CallFunction|CloseSwingGate)
  (Utilities|FlowControl|Gate false) ; enters at Close
)

(event EventBegin/EndSwing
  (params (Begin :type Boolean))
  (if Begin ; If a swing has started
    (Utilities|FlowControl|Gate false ; Allows us to disable a weapon\n(Like when the owner dies)
      (:Exit
        (CallFunction|OpenSwingGate)))
    (else
      (CallFunction|CloseSwingGate) ; Otherwise stop swinging
    )))

(event EventTick
  (params (DeltaSeconds :type Float%20%28single-precision%29))
  (Utilities|FlowControl|Gate true
    (:Exit
      (CallFunction|DamageCheck))))

(event EventBeginPlay
  (Utilities|Array|Add (Variables|Default|GetHitActors) (Actor|GetParentActor)) ; Adding the parent to the list of hit\nactors means we won't hit it during\nswings
)

(fn ConstructionScript
  (Utilities|Array|Add (Variables|Default|GetHitActors) self))

(fn DamageCheck
  (bind _returnvalue (Actor|GetParentActor))
  (bind _outhit (CallFunction|CollisionTrace)) ; Check if anything collides with\nthe sword
  (bind _output_get (LocalVariables|SetCollisionHit _outhit))
  (if (.bBlockingHit (Collision|BreakHitResult _output_get)) ; If anything was hit by the trace
    (LocalVariables|SetHitActor (.HitActor (Collision|BreakHitResult _output_get)))
    (bind _dead (Class|BPPawnInteractionInterface|GetIsDead(Message) (LocalVariables|GetHitActor)))
    (if _dead ; If the hit actor is already dead
      (Utilities|Array|Add (Variables|Default|GetHitActors) (LocalVariables|GetHitActor)) ; Add it to the list of hit actors to stop multiple hits in one swing
      (else
        (Game|Damage|ApplyPointDamage (LocalVariables|GetHitActor) (+ (Variables|Default|GetBaseDamage) (Variables|Default|GetDamageAddition)) (* (.Normal (Collision|BreakHitResult (LocalVariables|GetCollisionHit))) -1.0) (LocalVariables|GetCollisionHit) (Game|GetInstigatorController _returnvalue) _returnvalue "/Script/Engine.DamageType") ; Applies damage to the hit actor
        (bind _aspawn (Utilities|Casting|CastToPawn (LocalVariables|GetHitActor)) ; If the hit actor is a pawn
          (:then
            (bind _bleeds (Class|BPPawnInteractionInterface|ActorCanBleed(Message) _aspawn))
            (if (not _bleeds) ; If the actor cannot bleed
              _
              (else
                (Effects|SpawnEmitteratLocation "/Game/DarkRPGTemplate/Particles/PS_BloodSpurt.PS_BloodSpurt" (.Location (Collision|BreakHitResult (LocalVariables|GetCollisionHit))) (* (Math|Conversions|RotationFromXVector (.Normal (Collision|BreakHitResult (LocalVariables|GetCollisionHit)))) -1.0)) ; Otherwise spawn a blood spurt
              ))
            (Audio|PlaySoundatLocation "/Game/DarkRPGTemplate/Audio/Cues/SC_GoreCue.SC_GoreCue" (.Location (Collision|BreakHitResult (LocalVariables|GetCollisionHit))))
            (bind _dead_2 (Class|BPPawnInteractionInterface|GetIsDead(Message) (LocalVariables|GetHitActor)))
            (if _dead_2 ; If the actor has been killed
              (bind _xpworth (Class|BPPawnInteractionInterface|GetXPWorth(Message) (LocalVariables|GetHitActor)))
              (Class|BPPawnInteractionInterface|AddXP(Message) (Components|GetOwner (Transformation|GetAttachParent (Variables|Default|GetWeaponMesh))) _xpworth) ; Add the XP to the player
            )
            (Utilities|Array|Add (Variables|Default|GetHitActors) (LocalVariables|GetHitActor)) ; Then add the hit actor to the array\nso they don't get hit more than once\nin a single swing
          )
          (:CastFailed
            (bind _asbp_shield (Utilities|Casting|CastToBP_Shield (LocalVariables|GetHitActor)) ; If the hit actor is a shield
              (:then
                (if (Variables|/Game/DarkRPGTemplate/Blueprints/Armour/Shields/BP_Shield.BP_Shield_C|GetActive _asbp_shield) ; And it is active
                  (CallFunction|ImpactSolidObject (.Location (Collision|BreakHitResult (LocalVariables|GetCollisionHit)))) ; Impact a solid object
                  (CallFunction|Begin/EndSwing false) ; And stop swinging
                ))
              (:CastFailed
                (CallFunction|ImpactSolidObject (.Location (Collision|BreakHitResult (LocalVariables|GetCollisionHit)))) ; Otherwise just impact solid object
              ))))))))

(fn CollisionTrace
  (Utilities|Array|AddUnique (Variables|Default|GetHitActors) (Variables|Default|GetPlayerShield)) ; (Only matters for player's weapon)
  (if (Variables|Default|GetLineTrace) ; If this weapon should use a line\nfor tracing
    (bind _outhit (Collision|LineTraceByChannel (Transformation|GetWorldLocation (Variables|Default|GetDamageTrace01)) (Transformation|GetWorldLocation (Variables|Default|GetDamageTrace02)) "TraceTypeQuery3" false (Variables|Default|GetHitActors) "None"))
    (return _outhit)
    (else
      (bind _outhit_2 (Collision|SphereTraceByChannel (Transformation|GetWorldLocation (Variables|Default|GetDamageTrace01)) (Transformation|GetWorldLocation (Variables|Default|GetDamageTrace02)) (Variables|Default|GetSphereTraceRadius) "TraceTypeQuery3" false (Variables|Default|GetHitActors) "None"))
      (return _outhit_2))))

(fn ImpactSolidObject
  (params (HitLocation :type Vector))
  (Audio|PlaySoundatLocation "/Game/DarkRPGTemplate/Audio/Cues/SC_MetalImpactCue.SC_MetalImpactCue" HitLocation)
  (Class|BPPawnInteractionInterface|Stagger(Message) (Components|GetOwner (Transformation|GetAttachParent (Variables|Default|GetWeaponMesh))))
  (CallFunction|Begin/EndSwing false))

(fn ActorCanBleed
  (return false))

(fn AddtoUserInventory
  (params (InventoryItem :type BP%20Inventory%20Item%20Class%20Reference))
  (return false))

(fn Begin/EndPray
  (params (Begin :type Boolean))
  (return 0.0))

(fn GetFaction
  (return "NewEnumerator0"))

(fn GetIsDead
  (return false))

(fn GetTorsoMontage
  (return false))

(fn GetWeapon
  (return 0))

(fn GetXPWorth
  (return 0))