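; Blueprint function library of shared helpers for the Dark RPG template.
; GetClosest searches an actor list for the one nearest a source actor, and DetermineStats linearly converts Agility, Vitality and Strength into max stamina, max health and bonus damage.
; Two interp functions each move an actor or component one delta-time step toward a target location and/or rotation, returning whether it has arrived within tolerance, so they suit repeated per-frame calls.
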(fn GetClosest
  (params (Actors :type Array%20of%20Actor%20Object%20References) (SourceActor :type Actor%20Object%20Reference))
  (LocalVariables|SetSelfActor SourceActor)
  (for _array_element Actors ; Loop through the input actors
    (if (> (LocalVariables|GetCurrentMinDistance) (Transformation|GetDistanceTo _array_element (LocalVariables|GetSelfActor))) ; If the distance from the current closest\nactor is less than the current actor in\nthe loop
      (LocalVariables|SetCurrentMin _array_element) ; Set the current closest actor\nto the current loop actor
      (LocalVariables|SetCurrentMinDistance (Transformation|GetDistanceTo _array_element (LocalVariables|GetSelfActor)))))
  (return (LocalVariables|GetCurrentMin)) ; Once loop is finished,\nreturn the closest found\nactor
)

(fn InterpActortoLocationandRotation
  (params (Actor :type Actor%20Object%20Reference) (Location :type Vector) (Rotation :type Rotator) (InterpSpeed :type Float%20%28single-precision%29) (InterpRotation :type Boolean) (InterpLocation :type Boolean))
  ;[1 1 1] Save as local variables for use later
  (LocalVariables|SetTargetActor Actor)
  (LocalVariables|SetTargetLocation Location)
  (LocalVariables|SetTargetRotation Rotation)
  (LocalVariables|SetTargetInterpSpeed InterpSpeed)
  (LocalVariables|SetInterpRot InterpRotation)
  (LocalVariables|SetInterpLoc InterpLocation)
  (if (not (LocalVariables|GetInterpLoc)) ; If we should not interp location
    _
    (else
      (Transformation|SetActorLocation (LocalVariables|GetTargetActor) (Math|Interpolation|VInterpTo (Transformation|GetActorLocation (LocalVariables|GetTargetActor)) (LocalVariables|GetTargetLocation) (Utilities|Time|GetWorldDeltaSeconds (LocalVariables|GetTargetActor)) (LocalVariables|GetTargetInterpSpeed)) false false) ; Otherwise, update the location of the target actor
    ))
  (if (not (LocalVariables|GetInterpRot)) ; Same but with rotation
    _
    (else
      (Transformation|SetActorRotation (LocalVariables|GetTargetActor) (Math|Interpolation|RInterpTo (Transformation|GetActorRotation (LocalVariables|GetTargetActor)) (LocalVariables|GetTargetRotation) (Utilities|Time|GetWorldDeltaSeconds (LocalVariables|GetTargetActor)) (LocalVariables|GetTargetInterpSpeed)))))
  (return (and (select (LocalVariables|GetInterpLoc) (Math|Vector|Equal(Vector) (Transformation|GetActorLocation (LocalVariables|GetTargetActor)) (LocalVariables|GetTargetLocation) 0.0001) true) (select (LocalVariables|GetInterpRot) (Math|Rotator|Equal(Rotator) (Transformation|GetActorRotation (LocalVariables|GetTargetActor)) (LocalVariables|GetTargetRotation) 0.0001) true))) ; Return if the target actor is at the input target location/rotation
)

(fn DetermineStats
  (params (Stats :type Player%20Stats%20Structure))
  (bind _output_get (LocalVariables|SetLocalPlayerStats Stats))
  (LocalVariables|SetLocalMaxStamina (+ (* (Utilities|Struct|BreakPlayerStats _output_get) 15.0) 4e+01))
  (LocalVariables|SetLocalMaxHealth (+ (* (Utilities|Struct|BreakPlayerStats (LocalVariables|GetLocalPlayerStats)) 15.0) 4e+01))
  (LocalVariables|SetLocalDamageAddition (* (Utilities|Struct|BreakPlayerStats (LocalVariables|GetLocalPlayerStats)) 6.0))
  (return (LocalVariables|GetLocalMaxHealth) (LocalVariables|GetLocalMaxStamina) (LocalVariables|GetLocalDamageAddition)))

(fn InterpComponenttoLocationandRotation
  (params (Component :type Scene%20Component%20Object%20Reference) (Location :type Vector) (Rotation :type Rotator) (InterpSpeed :type Float%20%28single-precision%29) (InterpRotation :type Boolean) (InterpLocation :type Boolean))
  (LocalVariables|SetTargetComponent Component)
  (LocalVariables|SetTargetLocation Location)
  (LocalVariables|SetTargetRotation Rotation)
  (LocalVariables|SetTargetInterpSpeed InterpSpeed)
  (LocalVariables|SetInterpRot InterpRotation)
  (LocalVariables|SetInterpLoc InterpLocation)
  (if (not (LocalVariables|GetInterpLoc))
    _
    (else
      (Transformation|SetWorldLocation (LocalVariables|GetTargetComponent) (Math|Interpolation|VInterpTo (Transformation|GetWorldLocation (LocalVariables|GetTargetComponent)) (LocalVariables|GetTargetLocation) (Utilities|Time|GetWorldDeltaSeconds (LocalVariables|GetTargetComponent)) (LocalVariables|GetTargetInterpSpeed)) false false)))
  (if (not (LocalVariables|GetInterpRot))
    _
    (else
      (Transformation|SetWorldRotation (LocalVariables|GetTargetComponent) (Math|Interpolation|RInterpTo (Transformation|GetWorldRotation (LocalVariables|GetTargetComponent)) (LocalVariables|GetTargetRotation) (Utilities|Time|GetWorldDeltaSeconds (LocalVariables|GetTargetComponent)) (LocalVariables|GetTargetInterpSpeed)) false false)))
  (return (and (select (LocalVariables|GetInterpLoc) (Math|Vector|Equal(Vector) (Transformation|GetWorldLocation (LocalVariables|GetTargetComponent)) (LocalVariables|GetTargetLocation) 0.01) true) (select (LocalVariables|GetInterpRot) (Math|Rotator|Equal(Rotator) (Transformation|GetWorldRotation (LocalVariables|GetTargetComponent)) (LocalVariables|GetTargetRotation) 0.01) true))))