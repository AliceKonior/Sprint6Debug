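; Base buff Blueprint in the Dark RPG template that times how long a buff lasts on its owner.
; On BeginPlay it waits for Duration, then sends EndBuffMessage to the owner with itself as the argument, leaving the cleanup to the owner.
; The remaining functions, such as faction, death, weapon and XP queries, are stubs that return defaults, and the file applies no buff effect itself.
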(event EventBeginPlay
  (Utilities|FlowControl|Delay (Variables|Default|GetDuration))
  (Class|BPPawnInteractionInterface|EndBuff(Message) (Components|GetOwner) self))

(fn ConstructionScript)

(fn ActorCanBleed
  (return false))

(fn AddtoUserInventory
  (params (InventoryItem :type BP%20Inventory%20Item%20Class%20Reference))
  (return false))

(fn Begin/EndPray
  (params (Begin :type Boolean))
  (return 0.0))

(fn GetFaction
  (return "NewEnumerator0"))

(fn GetIsDead
  (return false))

(fn GetTorsoMontage
  (return false))

(fn GetWeapon
  (return 0))

(fn GetXPWorth
  (return 0))