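; Blueprint interface for the Dark RPG template that lets objects interact with pawns without casting to their classes.
; It declares calls for using and inventory pickup, interaction enter and exit, health, stamina, XP and skillpoints, and timed stat buffs.
; It also covers combat and gear, including swings, stagger, shield hits, bleeding and equipment changes, plus altar praying and queries for faction, death and weapon.
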(fn Use
  (params (User :type Pawn%20Object%20Reference)))

(fn AddtoUserInventory
  (params (InventoryItem :type BP%20Inventory%20Item%20Class%20Reference))
  (return false))

(fn Entered
  (params (Object :type BP%20Usable%20Object%20Object%20Reference) (Action :type String)))

(fn Exited
  (params (Object :type BP%20Usable%20Object%20Object%20Reference)))

(fn AffectActorHealth
  (params (AffectAmount :type Float%20%28single-precision%29)))

(fn GetFaction
  (return "NewEnumerator0"))

(fn GetIsDead
  (return false))

(fn Begin/EndSwing
  (params (Begin :type Boolean)))

(fn GetWeapon
  (return 0))

(fn ActorCanMove
  (params (CanMove :type Boolean)))

(fn AffectActorStamina
  (params (AffectAmount :type Float%20%28single-precision%29)))

(fn Begin/EndPray
  (params (Begin :type Boolean))
  (return 0.0))

(fn AddXP
  (params (Amount :type Integer)))

(fn GetXPWorth
  (return 0))

(fn Stagger)

(fn EquipArmour
  (params (ArmourStats :type Armour%20Stats%20Structure)))

(fn GetTorsoMontage
  (return false))

(fn ShieldHit)

(fn EquipNewWeapon
  (params (WeaponClass :type BP%20Weapon%20Class%20Reference)))

(fn EquipNewShield
  (params (ShieldClass :type BP%20Shield%20Class%20Reference)))

(fn ActorCanBleed
  (return false))

(fn AddSkillpoints
  (params (Skillpoints :type Integer)))

(fn SetLastAltar
  (params (Altar :type BP%20Altar%20Object%20Reference)))

(fn SheatheWeapon)

(fn UnequipArmour
  (params (Slot :type ArmourSlot%20Enum :default "NewEnumerator0")))

(fn EndBuff
  (params (BuffToEnd :type BP%20Buff%20Object%20Reference)))

(fn Buff
  (params (Stat :type Stat%20Enum :default "NewEnumerator0") (AffectAmount :type Float%20%28single-precision%29) (Duration :type Float%20%28single-precision%29)))