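; BP_UsableObject is an interactable world object that tells actors when they can use it.
; Overlapping its UseTrigger sends the other actor EnteredMessage with the object and its ActionText, and leaving sends ExitedMessage.
; The remaining functions, covering bleeding, inventory, praying, faction, death, montage, weapon and XP, are stubs returning defaults, and the construction script is empty.
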(event OnComponentBeginOverlap(UseTrigger)
  (params (OverlappedComponent :type Primitive%20Component%20Object%20Reference) (OtherActor :type Actor%20Object%20Reference) (OtherComp :type Primitive%20Component%20Object%20Reference) (OtherBodyIndex :type Integer) (bFromSweep :type Boolean) (SweepResult :type Hit%20Result%20Structure%20%28by%20ref%29))
  (Class|BPPawnInteractionInterface|Entered(Message) OtherActor self (Variables|Default|GetActionText)) ; Notify the overlapping actor that they have entered the volume
)

(event OnComponentEndOverlap(UseTrigger)
  (params (OverlappedComponent :type Primitive%20Component%20Object%20Reference) (OtherActor :type Actor%20Object%20Reference) (OtherComp :type Primitive%20Component%20Object%20Reference) (OtherBodyIndex :type Integer))
  (Class|BPPawnInteractionInterface|Exited(Message) OtherActor self) ; Then notify when they have exited it
)

(fn ConstructionScript)

(fn ActorCanBleed
  (return false))

(fn AddtoUserInventory
  (params (InventoryItem :type BP%20Inventory%20Item%20Class%20Reference))
  (return false))

(fn Begin/EndPray
  (params (Begin :type Boolean))
  (return 0.0))

(fn GetFaction
  (return "NewEnumerator0"))

(fn GetIsDead
  (return false))

(fn GetTorsoMontage
  (return false))

(fn GetWeapon
  (return 0))

(fn GetXPWorth
  (return 0))