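; BP_DeathLocation is a usable actor that holds the XP and skillpoints lost on death so they can be reclaimed.
; Use sends the stored XP and skillpoints to the user through message calls, then destroys the actor.
; On BeginPlay it binds to the player's death dispatcher and destroys itself if the player dies again, leaving one life to recover the loss.
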(event Custom|PlayerDeath
  (Actor|DestroyActor) ; When the player dies, destroy self. This means they only have one life to reach lost XP
)

(event EventUse
  (params (User :type Pawn%20Object%20Reference))
  (Class|BPPawnInteractionInterface|AddXP(Message) User (Variables|Default|GetXP)) ; Add the lost XP to the user
  (Class|BPPawnInteractionInterface|AddSkillpoints(Message) User (Variables|Default|GetSkillpoints)) ; Add the lost Skillpoints to the user
  (Actor|DestroyActor) ; Once XP and Skillpoints have been returned, destroy this actor
)

(event EventBeginPlay
  (bind _asbp_player (Utilities|Casting|CastToBP_Player (Game|GetPlayerCharacter 0)))
  (EventDispatchers|BindEventtoPlayerDeath _asbp_player (delegate Custom|PlayerDeath)) ; When spawned, bind PlayerDeath\nto Player's death dispatch.
)

(fn ConstructionScript
  (|CallParentFunction))