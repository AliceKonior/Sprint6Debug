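; BP_ArmourSet is a container for a character's six armour slots (helmet, cuirass, greaves, gauntlets, cape, pauldrons), each a child actor.
; Equip and unequip calls select the slot's child actor by slot type and forward a message to it.
; It sums armour values across slots and returns the pieces as an array.
; SetMasterPose binds each piece's mesh to a supplied skeletal mesh, intended as the player's, so armour follows its animation.
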(fn ConstructionScript)

(fn SetMasterPose
  (params (SkeletalMeshComp :type Skeletal%20Mesh%20Component%20Object%20Reference))
  (LocalVariables|SetLocalSkelMeshComp SkeletalMeshComp)
  (for _array_element (Utilities|Array|MakeArray (Variables|Default|GetHelmetSlot) (Variables|Default|GetCuirassSlot) (Variables|Default|GetGreavesSlot) (Variables|Default|GetGauntletsSlot) (Variables|Default|GetCapeSlot) (Variables|Default|GetPauldronsSlot)) ; Loop through each slot
    (bind _asbp_armour_piece (Utilities|Casting|CastToBP_ArmourPiece (Variables|/Script/Engine.ChildActorComponent|GetChildActor _array_element))) ; Cast so we can get the mesh component
    (Class|SkinnedMeshComponent|SetMasterPoseComponent (Variables|/Game/DarkRPGTemplate/Blueprints/Armour/BP_ArmourPiece.BP_ArmourPiece_C|GetMesh _asbp_armour_piece) (LocalVariables|GetLocalSkelMeshComp)) ; Assign the armour mesh to the master\nmesh (Which should be the character mesh\nof the player)
  ))

(fn GetArmourActors
  (for _array_element (Utilities|Array|MakeArray (Variables|/Script/Engine.ChildActorComponent|GetChildActor (Variables|Default|GetHelmetSlot)) (Variables|/Script/Engine.ChildActorComponent|GetChildActor (Variables|Default|GetCuirassSlot)) (Variables|/Script/Engine.ChildActorComponent|GetChildActor (Variables|Default|GetPauldronsSlot)) (Variables|/Script/Engine.ChildActorComponent|GetChildActor (Variables|Default|GetGreavesSlot)) (Variables|/Script/Engine.ChildActorComponent|GetChildActor (Variables|Default|GetGauntletsSlot)) (Variables|/Script/Engine.ChildActorComponent|GetChildActor (Variables|Default|GetCapeSlot)))
    (bind _asbp_armour_piece (Utilities|Casting|CastToBP_ArmourPiece _array_element))
    (Utilities|Array|Add (LocalVariables|GetLocalArmour) _asbp_armour_piece) ; Add all the contents of the\narmour slots to an array
  )
  (return (LocalVariables|GetLocalArmour)) ; Once all are added, return the array
)

(fn Equip/ReplaceArmour
  (params (ArmourStats :type Armour%20Stats%20Structure))
  (bind _success (Class|BPArmourInterface|Equip/ReplaceArmour(Message) (Utilities|Select :Index (Utilities|Struct|BreakArmourStats ArmourStats) :NewEnumerator0 (Variables|/Script/Engine.ChildActorComponent|GetChildActor (Variables|Default|GetHelmetSlot)) :NewEnumerator1 (Variables|/Script/Engine.ChildActorComponent|GetChildActor (Variables|Default|GetCuirassSlot)) :NewEnumerator2 (Variables|/Script/Engine.ChildActorComponent|GetChildActor (Variables|Default|GetGreavesSlot)) :NewEnumerator3 (Variables|/Script/Engine.ChildActorComponent|GetChildActor (Variables|Default|GetGauntletsSlot)) :NewEnumerator4 (Variables|/Script/Engine.ChildActorComponent|GetChildActor (Variables|Default|GetCapeSlot)) :NewEnumerator5 (Variables|/Script/Engine.ChildActorComponent|GetChildActor (Variables|Default|GetPauldronsSlot))) ArmourStats))
  (return _success))

(fn GetArmourValue
  (LocalVariables|SetLocalArmourValue 0.0) ; Make sure armour value is at 0 before\ncalculating
  (for _array_element (Utilities|Array|MakeArray (Variables|/Script/Engine.ChildActorComponent|GetChildActor (Variables|Default|GetHelmetSlot)) (Variables|/Script/Engine.ChildActorComponent|GetChildActor (Variables|Default|GetCuirassSlot)) (Variables|/Script/Engine.ChildActorComponent|GetChildActor (Variables|Default|GetGreavesSlot)) (Variables|/Script/Engine.ChildActorComponent|GetChildActor (Variables|Default|GetGauntletsSlot)) (Variables|/Script/Engine.ChildActorComponent|GetChildActor (Variables|Default|GetCapeSlot)) (Variables|/Script/Engine.ChildActorComponent|GetChildActor (Variables|Default|GetPauldronsSlot))) ; Loops through each armour\npiece
    (bind _armourvalue (Class|BPArmourInterface|GetArmourValue(Message) _array_element))
    (LocalVariables|SetLocalArmourValue (+ _armourvalue (LocalVariables|GetLocalArmourValue))) ; Add each armour value to the\ntotal
  )
  (return (LocalVariables|GetLocalArmourValue)) ; Once calculated, return total armour value
)

(fn UnequipArmour
  (params (SlotToUnequip :type ArmourSlot%20Enum :default "NewEnumerator0"))
  (bind _success (Class|BPArmourInterface|UnequipArmour(Message) (Utilities|Select :Index SlotToUnequip :NewEnumerator0 (Variables|/Script/Engine.ChildActorComponent|GetChildActor (Variables|Default|GetHelmetSlot)) :NewEnumerator1 (Variables|/Script/Engine.ChildActorComponent|GetChildActor (Variables|Default|GetCuirassSlot)) :NewEnumerator2 (Variables|/Script/Engine.ChildActorComponent|GetChildActor (Variables|Default|GetGreavesSlot)) :NewEnumerator3 (Variables|/Script/Engine.ChildActorComponent|GetChildActor (Variables|Default|GetGauntletsSlot)) :NewEnumerator4 (Variables|/Script/Engine.ChildActorComponent|GetChildActor (Variables|Default|GetCapeSlot)) :NewEnumerator5 (Variables|/Script/Engine.ChildActorComponent|GetChildActor (Variables|Default|GetPauldronsSlot))) SlotToUnequip))
  (return _success))