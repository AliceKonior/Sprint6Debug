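; BP_ArmourPiece represents one armour slot, holding its stats, skeletal mesh and protection value.
; Equipping sends an unequip message for the slot to the owner of the mesh's attach parent (the armour set), then stores new stats and refreshes the mesh.
; Unequipping checks slot and set state, then clears everything but the slot.
; Meshes using cloth in section 0 are routed to player 0's Cape component instead of the piece's own mesh.
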(fn ConstructionScript)

(fn UnequipSelf
  (if (Class|SkeletalMesh|IsSectionUsingCloth (Utilities|Struct|BreakArmourStats (Variables|Default|GetArmourStats)) 0 true)
    (bind _asbp_player (Utilities|Casting|CastToBP_Player (Game|GetPlayerCharacter 0)))
    (Class|SkinnedMeshComponent|SetSkeletalMesh (Variables|/Game/DarkRPGTemplate/Blueprints/Player/BP_Player.BP_Player_C|GetCape _asbp_player) 0 true))
  (Variables|Default|SetArmourStats (Utilities|Struct|MakeArmourStats (Utilities|Struct|BreakArmourStats (Variables|Default|GetArmourStats)) 0 0.0)) ; Reset all variables except\nslot
  (CallFunction|UpdateMesh) ; Update the mesh component\n(Will change to no mesh given\nArmourStats  Mesh variable)
  (Variables|Default|SetIsSet false)
  (return))

(fn UpdateMesh
  (if (Class|SkeletalMesh|IsSectionUsingCloth (Utilities|Struct|BreakArmourStats (Variables|Default|GetArmourStats)) 0 true)
    (bind _asbp_player (Utilities|Casting|CastToBP_Player (Game|GetPlayerCharacter 0)))
    (Class|SkinnedMeshComponent|SetSkeletalMesh (Variables|/Game/DarkRPGTemplate/Blueprints/Player/BP_Player.BP_Player_C|GetCape _asbp_player) (Utilities|Struct|BreakArmourStats (Variables|Default|GetArmourStats)) true)
    (else
      (Class|SkinnedMeshComponent|SetSkeletalMesh (Variables|Default|GetMesh) (Utilities|Struct|BreakArmourStats (Variables|Default|GetArmourStats)) true))))

(fn Equip/ReplaceArmour
  (params (ArmourStats :type Armour%20Stats%20Structure))
  (LocalVariables|SetLocalArmourStats ArmourStats)
  (Class|BPArmourInterface|UnequipArmour(Message) (Components|GetOwner (Transformation|GetAttachParent (Variables|Default|GetMesh))) (Utilities|Struct|BreakArmourStats (Variables|Default|GetArmourStats))) ; First unequip the current armour
  (Variables|Default|SetIsSet true)
  (Variables|Default|SetArmourStats (LocalVariables|GetLocalArmourStats)) ; Then update the armour \nstats to the input armour\nstats
  (CallFunction|UpdateMesh)
  (return true))

(fn GetArmourValue
  (return (Utilities|Struct|BreakArmourStats (Variables|Default|GetArmourStats))))

(fn UnequipArmour
  (params (SlotToUnequip :type ArmourSlot%20Enum :default "NewEnumerator0"))
  (if (and (Utilities|Enum|Equal(Enum) SlotToUnequip (Utilities|Struct|BreakArmourStats (Variables|Default|GetArmourStats))) (Variables|Default|GetIsSet)) ; Make sure we have the right\nslot chosen and the armour \npiece is set
    (CallFunction|UnequipSelf)
    (return true)
    (else
      (return false))))