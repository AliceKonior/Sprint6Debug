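; BP_Shield is a shield actor in the Dark RPG template that reacts when it takes damage.
; While Active, its AnyDamage event sends ShieldHitMessage to its parent actor, the player, to cause knockback.
; The other functions, covering bleeding, inventory, faction, death, weapon and XP queries, are stubs returning defaults, so the shield neither bleeds nor grants XP.
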(event Game|Damage|EventAnyDamage
  (params (Damage :type Float%20%28single-precision%29) (DamageType :type Damage%20Type%20Object%20Reference) (InstigatedBy :type Controller%20Object%20Reference) (DamageCauser :type Actor%20Object%20Reference))
  (if (Variables|Default|GetActive) ; If it is active
    (Class|BPPawnInteractionInterface|ShieldHit(Message) (Actor|GetParentActor)) ; Call shield hit on the player, causing knockback
  ))

(fn ConstructionScript)

(fn ActorCanBleed
  (return false))

(fn AddtoUserInventory
  (params (InventoryItem :type BP%20Inventory%20Item%20Class%20Reference))
  (return false))

(fn Begin/EndPray
  (params (Begin :type Boolean))
  (return 0.0))

(fn GetFaction
  (return "NewEnumerator0"))

(fn GetIsDead
  (return false))

(fn GetTorsoMontage
  (return false))

(fn GetWeapon
  (return 0))

(fn GetXPWorth
  (return 0))